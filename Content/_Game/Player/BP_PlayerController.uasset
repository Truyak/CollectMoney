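; Player controller that sets up Enhanced Input and handles pausing and level progression.
; On BeginPlay it adds the default mapping context, caches the HUD and loads the save slot.
; PauseEvent toggles game pause, cursor and input mode through the HUD's pause widget, backing out of settings first.
; NextLevelLoad parses the current level name's number to open the next Level_N map, returning to the main menu after the last.
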(event Custom|Event%20NextLevelLoad
  (bind _returnvalue (Game|GetCurrentLevelName true))
  (bind _output_get (Variables|Default|SetPrevLevelOrder (Math|Conversions|ToInteger(Byte) (.RightS (Utilities|String|Split _returnvalue "_")))))
  (if (!= _output_get (Variables|Default|GetMaxLevel))
    (Game|OpenLevel(byName) (Utilities|String|StringToName (Utilities|String|Append "Level_" (Utilities|String|ToString(Integer) (+ _output_get 1)))))
    (Input|SetInputModeGameOnly self false)
    (Variables|Default|SetbShowMouseCursor false)
    (else
      (Game|OpenLevel(byObjectReference) "/Game/_Game/Level/MainMenu.MainMenu"))))

(event Custom|PauseEvent
  (bind _bp_hud (Variables|Default|GetBP_HUD))
  (bind _wb_pausemenuui (Variables|/Game/_Game/Player/BP_HUD.BP_HUD_C|GetWB_PauseMenuUI _bp_hud))
  (if (Variables|Default|GetbGamePaused)
    (if (Variables|Default|GetbIsSettingsMenuActive)
      (Widget|RemovefromParent (Variables|/Game/_Game/Player/BP_HUD.BP_HUD_C|GetWB_SettingsUI (Variables|Default|GetBP_HUD)))
      (UserInterface|Viewport|AddtoViewport _wb_pausemenuui 0)
      (Input|SetInputModeUIOnly self _wb_pausemenuui "DoNotLock" false)
      (Variables|Default|SetbIsSettingsMenuActive false)
      (else
        (Widget|RemovefromParent _wb_pausemenuui)
        (Game|SetGamePaused false)
        (Variables|Default|SetbShowMouseCursor false)
        (Input|SetInputModeGameOnly self false)
        (Variables|Default|SetbGamePaused false)))
    (else
      (Game|SetGamePaused true)
      (Variables|Default|SetbShowMouseCursor true)
      (UserInterface|Viewport|AddtoViewport _wb_pausemenuui 0)
      (Input|SetInputModeUIOnly self _wb_pausemenuui "DoNotLock" false)
      (Variables|Default|SetbGamePaused true))))

(event EventBeginPlay
  (bind _returnvalue (PlayerController|LocalPlayerSubsystems|GetEnhancedInputLocalPlayerSubsystem))
  (Utilities|IsValid _returnvalue
    (:Is%20Valid
      (Input|AddMappingContext _returnvalue "/Game/_Game/Player/Input/IA_DefaultMap.IA_DefaultMap" 0 "(bIgnoreAllPressedKeysUntilRelease=True,bForceImmediately=False,bNotifyUserSettings=False)")
      (bind _asbp_hud (Utilities|Casting|CastToBP_HUD (HUD|GetHUD))
        (:then
          _)
        (:CastFailed
          _))
      (Variables|Default|SetBP_HUD _asbp_hud)
      (bind _returnvalue_2 (SaveGame|LoadGamefromSlot (Variables|Default|GetSaveSlot)))
      (bind _asbp_save (Utilities|Casting|CastToBP_Save _returnvalue_2))
      (Variables|Default|SetBP%20Save _asbp_save))))

(event EventTick
  (params (DeltaSeconds :type Float%20%28single-precision%29)))

(fn ConstructionScript)