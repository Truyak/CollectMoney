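; Manager that builds a random parkour path by choosing one of four colored actors (yellow, red, green, blue) for each row.
; Per-color checks compare the candidate's index with the number parsed from the previous actor's display name, accepting only certain offsets.
; Rejected picks narrow the random interval from either side until one fits.
; The finished path gets query-and-physics collision and is passed to BP_PlayerCharacter as a new parkour entrance.
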(event Custom|Randomize
  (bind _output_get (Variables|Default|Seti 0))
  (while (< _output_get (Variables|Default|GetTotalLength))
    (bind _output_get_2 (Variables|Default|SetRandomizedInteger (Utilities|RandomActor)))
    (Variables|Default|SetRandomizedIndex (+ _output_get_2 (* 4 (Variables|Default|Geti))))
    (if (== (Variables|Default|Geti) 0)
      (bind _actor (CallFunction|GetActorbyInteger :!label _label))
      (Utilities|Array|SetArrayElem (Variables|Default|GetCorrectPath) (Variables|Default|Geti) _actor true)
      (Variables|Default|SetbCanAssign false)
      (Variables|Default|SetbIsLefter false)
      (Variables|Default|SetbIsRighter false)
      (Math|Integer|IncrementInt (Variables|Default|Geti))
      (else
        (switch int (Variables|Default|GetRandomizedInteger)
          (:0
            (CallFunction|YellowCheck))
          (:1
            (CallFunction|RedCheck))
          (:2
            (CallFunction|GreenCheck))
          (:3
            (CallFunction|BlueCheck)))
        (if (Variables|Default|GetbCanAssign)
          (Variables|Default|SetRandomIntervalMax 3)
          (Variables|Default|SetRandomIntervalMin 0)
          (goto _label)
          (else
            (if (Variables|Default|GetbIsRighter)
              (Variables|Default|SetRandomIntervalMin (+ (Variables|Default|GetRandomIntervalMin) 1)))
            (if (Variables|Default|GetbIsLefter)
              (Variables|Default|SetRandomIntervalMax (- (Variables|Default|GetRandomIntervalMax) 1))))))))
  (for _array_element (Variables|Default|GetCorrectPath)
    (bind _asstatic_mesh_actor (Utilities|Casting|CastToStaticMeshActor _array_element))
    (Collision|SetCollisionEnabled (Variables|/Script/Engine.StaticMeshActor|GetStaticMeshComponent _asstatic_mesh_actor) "QueryAndPhysics"))
  (bind _asbp_player_character (Utilities|Casting|CastToBP_PlayerCharacter (Game|GetPlayerCharacter 0)))
  (Default|EventNewParkourEntrance _asbp_player_character (Variables|Default|GetCorrectPath)))

(event Custom|GreenCheck
  (bind _difference (CallFunction|GetDiff))
  (if (Math|Boolean|ORBoolean (== _difference 5) (== _difference 4) (== _difference 3))
    (Variables|Default|SetbCanAssign (Math|Boolean|ORBoolean (== _difference 5) (== _difference 4) (== _difference 3)))
    (else
      (Variables|Default|SetbIsLefter true))))

(event Custom|BlueCheck
  (bind _difference (CallFunction|GetDiff))
  (if (or (== _difference 4) (== _difference 5))
    (Variables|Default|SetbCanAssign (or (== _difference 4) (== _difference 5)))
    (else
      (Variables|Default|SetbIsLefter (> _difference 5)))))

(event Custom|RedCheck
  (bind _difference (CallFunction|GetDiff))
  (if (Math|Boolean|ORBoolean (== _difference 5) (== _difference 4) (== _difference 3))
    (Variables|Default|SetbCanAssign (Math|Boolean|ORBoolean (== _difference 5) (== _difference 4) (== _difference 3)))
    (else
      (Variables|Default|SetbIsRighter true))))

(event Custom|YellowCheck
  (bind _difference (CallFunction|GetDiff))
  (if (or (== _difference 4) (== _difference 3))
    (Variables|Default|SetbCanAssign (or (== _difference 4) (== _difference 3)))
    (else
      (Variables|Default|SetbIsRighter true))))

(event EventBeginPlay)

(fn ConstructionScript)

(fn GetDiff
  (return (- (Variables|Default|GetRandomizedIndex) (Math|Conversions|ToInteger(Byte) (.RightS (Utilities|String|Split (Utilities|GetDisplayName (Utilities|Array|Get(acopy) (Variables|Default|GetCorrectPath) (- (Variables|Default|Geti) 1))) "e"))))))

(fn GetActorbyInteger
  (switch int (Variables|Default|GetRandomizedInteger)
    (:0
      (return (Utilities|Array|Get(acopy) (Variables|Default|GetYellowActors) (/ (Variables|Default|GetRandomizedIndex) 4))))
    (:1
      (return (Utilities|Array|Get(acopy) (Variables|Default|GetRedActors) (/ (Variables|Default|GetRandomizedIndex) 4))))
    (:2
      (return (Utilities|Array|Get(acopy) (Variables|Default|GetGreenActors) (/ (Variables|Default|GetRandomizedIndex) 4))))
    (:3
      (return (Utilities|Array|Get(acopy) (Variables|Default|GetBlueActors) (/ (Variables|Default|GetRandomizedIndex) 4))))))