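; BP_CheckpointManager tracks which checkpoint is active and shares that state with the player character.
; On BeginPlay it caches the player and passes it the Checkpoints map.
; UpdateCheckpoint hides the first visible cursor, reveals the next, then flags the given checkpoint true and its predecessor false by key order before notifying the player.
; IsCheckpointSetted gates updates and is never reset within this Blueprint.
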(event Custom|Event%20Update%20Checkpoint
  (params (Setted%20Checkpoint :type Actor%20Object%20Reference))
  (bind _checkpointcursors (Variables|Default|GetCheckpointCursors))
  (bind _checkpoints (Variables|Default|GetCheckpoints))
  (if (not (Variables|Default|GetbIsCheckpointSetted))
    (bind (_array_element _array_index) (Utilities|Array|ForEachLoopwithBreak _checkpointcursors)
      (:LoopBody
        (if (not (Variables|/Script/Engine.Actor|GetbHidden _array_element))
          (Rendering|SetActorHiddenInGame _array_element true)
          (Rendering|SetActorHiddenInGame (Utilities|Array|Get(acopy) _checkpointcursors (+ _array_index 1)) false)
          (CallFunction|BreakLoop)))
      (:Completed
        (bind _keys (Utilities|Map|Keys _checkpoints))
        (for (_array_element_2 _array_index_2) _keys
          (if (== _array_element_2 Setted%20Checkpoint)
            (bind _keys_2 (Utilities|Map|Keys _checkpoints))
            (Utilities|Map|Add _checkpoints (Utilities|Array|Get(acopy) _keys_2 (- _array_index_2 1)) false)
            (Utilities|Map|Add _checkpoints (Utilities|Array|Get(acopy) _keys_2 _array_index_2) true)
            (Development|PrintString "Checkpoint Set")
            (Variables|Default|SetbIsCheckpointSetted true)
            (Default|EventUpdateCheckpointsSituation (Variables|Default|GetBP%20Player%20Character) _checkpoints)))))))

(event Custom|BreakLoop
  (bind _checkpointcursors (Variables|Default|GetCheckpointCursors))
  (bind _checkpoints (Variables|Default|GetCheckpoints))
  (Utilities|Array|ForEachLoopwithBreak _checkpointcursors) ; enters at Break
)

(event EventBeginPlay
  (bind _asbp_player_character (Utilities|Casting|CastToBP_PlayerCharacter (Game|GetPlayerCharacter 0)))
  (bind _output_get (Variables|Default|SetBP%20Player%20Character _asbp_player_character))
  (Default|EventUpdateCheckpointsSituation _output_get (Variables|Default|GetCheckpoints)))

(fn ConstructionScript)