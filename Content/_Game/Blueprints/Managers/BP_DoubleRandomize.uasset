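; Manager that randomly picks the left or right cube in each pair of carousel cubes at game start.
; On BeginPlay it walks the LeftSide and RightSide arrays by index, flips a coin and enables query and physics collision on the chosen BP_CarouselCubes mesh.
; The construction script takes the pair count from RightSide's length, and each pick prints a Turkish left/right debug label.
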(event EventBeginPlay
  (bind _output_get (Variables|Default|Seti 0))
  (while (< _output_get (Variables|Default|GetTotalLength))
    (switch int (Math|Random|RandomInteger 2)
      (:0
        (Development|PrintString "Sol" true true "(R=0.000000,G=0.660000,B=1.000000,A=1.000000)" 5e+01)
        (bind _asbp_carousel_cubes (Utilities|Casting|CastToBP_CarouselCubes (Utilities|Array|Get(acopy) (Variables|Default|GetLeftSide) (Variables|Default|Geti))))
        (Collision|SetCollisionEnabled (Variables|/Game/_Game/Blueprints/Environment/BP_CarouselCubes.BP_CarouselCubes_C|GetStaticMesh _asbp_carousel_cubes) "QueryAndPhysics"))
      (:1
        (Development|PrintString "Sağ" true true "(R=0.000000,G=0.660000,B=1.000000,A=1.000000)" 5e+01)
        (bind _asbp_carousel_cubes_2 (Utilities|Casting|CastToBP_CarouselCubes (Utilities|Array|Get(acopy) (Variables|Default|GetRightSide) (Variables|Default|Geti))))
        (Collision|SetCollisionEnabled (Variables|/Game/_Game/Blueprints/Environment/BP_CarouselCubes.BP_CarouselCubes_C|GetStaticMesh _asbp_carousel_cubes_2) "QueryAndPhysics")))
    (Math|Integer|IncrementInt (Variables|Default|Geti))))

(fn ConstructionScript
  (Variables|Default|SetTotalLength (Utilities|Array|Length (Variables|Default|GetRightSide))))