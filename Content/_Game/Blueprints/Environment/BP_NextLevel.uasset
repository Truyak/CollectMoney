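; Level exit trigger that completes the level when BP_PlayerCharacter overlaps its box.
; It loads BP_Save on BeginPlay, then on completion sets an IsLevelsUnlocked entry, indexed by the level name's numeric suffix minus one, and saves.
; It then pauses the game, shows the next-level widget from the player controller's HUD, and switches to UI-only input with a visible cursor.
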(event OnComponentBeginOverlap(Box)
  (params (OverlappedComponent :type Primitive%20Component%20Object%20Reference) (OtherActor :type Actor%20Object%20Reference) (OtherComp :type Primitive%20Component%20Object%20Reference) (OtherBodyIndex :type Integer) (bFromSweep :type Boolean) (SweepResult :type Hit%20Result%20Structure%20%28by%20ref%29))
  (if (== (Utilities|GetClass OtherActor) "/Game/_Game/Player/BP_PlayerCharacter.BP_PlayerCharacter_C")
    (CallFunction|FinishLevel)))

(event EventBeginPlay
  (bind _returnvalue (SaveGame|LoadGamefromSlot (Variables|Default|GetSaveSlot)))
  (bind _asbp_save (Utilities|Casting|CastToBP_Save _returnvalue))
  (Variables|Default|SetBP%20Save _asbp_save))

(event Collision|EventActorBeginOverlap
  (params (OtherActor :type Actor%20Object%20Reference)))

(event EventTick
  (params (DeltaSeconds :type Float%20%28single-precision%29)))

(fn ConstructionScript)

(fn UnlockNextLevel
  (bind _returnvalue (Game|GetCurrentLevelName true))
  (Utilities|Array|SetArrayElem (Variables|/Game/_Game/Save/BP_Save.BP_Save_C|GetbIsLevelsUnlocked (Variables|Default|GetBP%20Save)) (- (Math|Conversions|ToInteger(Byte) (.RightS (Utilities|String|Split _returnvalue "_"))) 1) true true)
  (SaveGame|SaveGametoSlot (Variables|Default|GetBP%20Save) (Variables|Default|GetSaveSlot)))

(fn FinishLevel
  (bind _returnvalue (Game|GetPlayerController 0))
  (CallFunction|UnlockNextLevel)
  (Game|SetGamePaused true)
  (bind _asbp_player_controller (Utilities|Casting|CastToBP_PlayerController (Game|GetPlayerController 0)))
  (UserInterface|Viewport|AddtoViewport (Variables|/Game/_Game/Player/BP_HUD.BP_HUD_C|GetWB_NextLevelUI (Variables|/Game/_Game/Player/BP_PlayerController.BP_PlayerController_C|GetBP_HUD _asbp_player_controller)) 0)
  (Input|SetInputModeUIOnly _returnvalue (Variables|/Game/_Game/Player/BP_HUD.BP_HUD_C|GetWB_NextLevelUI (Variables|/Game/_Game/Player/BP_PlayerController.BP_PlayerController_C|GetBP_HUD _asbp_player_controller)) "DoNotLock" false)
  (Variables|/Script/Engine.PlayerController|SetbShowMouseCursor _returnvalue true))