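; BP_LavaBlocks is an environment block that changes the player's health while they stand in its box collision.
; Overlap by BP_PlayerCharacter starts a looping timer, apparently driving the Damage event, and end overlap clears it.
; Damage calls the player character cached at BeginPlay, decreasing health for positive DamageAmount and healing otherwise, so one Blueprint serves both uses.
; The construction script applies the Material variable to the block mesh.
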(event OnComponentBeginOverlap(BoxCollision)
  (params (OverlappedComponent :type Primitive%20Component%20Object%20Reference) (OtherActor :type Actor%20Object%20Reference) (OtherComp :type Primitive%20Component%20Object%20Reference) (OtherBodyIndex :type Integer) (bFromSweep :type Boolean) (SweepResult :type Hit%20Result%20Structure%20%28by%20ref%29))
  (if (== (Utilities|GetClass OtherActor) "/Game/_Game/Player/BP_PlayerCharacter.BP_PlayerCharacter_C")
    (bind _returnvalue (Utilities|Time|SetTimerbyEvent (EventDispatchers|CreateEvent :!event Custom|Event%20Damage) 0.2 true))
    (Variables|Default|SetTimerEvent _returnvalue)))

(event OnComponentEndOverlap(BoxCollision)
  (params (OverlappedComponent :type Primitive%20Component%20Object%20Reference) (OtherActor :type Actor%20Object%20Reference) (OtherComp :type Primitive%20Component%20Object%20Reference) (OtherBodyIndex :type Integer))
  (if (== (Utilities|GetClass OtherActor) "/Game/_Game/Player/BP_PlayerCharacter.BP_PlayerCharacter_C")
    (Utilities|Time|ClearandInvalidateTimerbyHandle (Variables|Default|GetTimerEvent))))

(event Custom|Event%20Damage
  (bind _damageamount (Variables|Default|GetDamageAmount))
  (bind _bp_player_character (Variables|Default|GetBP%20Player%20Character))
  (if (<= _damageamount 0)
    (Default|EventIncreaseHealth _bp_player_character (* _damageamount -1))
    (else
      (Default|EventDecreaseHealth _bp_player_character _damageamount))))

(event EventBeginPlay
  (bind _asbp_player_character (Utilities|Casting|CastToBP_PlayerCharacter (Game|GetPlayerCharacter 0)))
  (Variables|Default|SetBP%20Player%20Character _asbp_player_character))

(fn ConstructionScript
  (Rendering|Material|SetMaterial (Variables|Default|GetLavaBlock) 0 (Variables|Default|GetMaterial)))