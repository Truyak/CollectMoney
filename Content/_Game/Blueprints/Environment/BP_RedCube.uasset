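; BP_RedCube is an environment Blueprint with a Box trigger that reacts to BP_PlayerCharacter.
; When the player's overlap begins and IsClickable is true, it prints a debug "Hello" and calls the Transfer event.
; Transfer calls Teleport on the Blueprint itself, not the player, targeting a point slightly above RedCube's world location.
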(event OnComponentBeginOverlap(Box)
  (params (OverlappedComponent :type Primitive%20Component%20Object%20Reference) (OtherActor :type Actor%20Object%20Reference) (OtherComp :type Primitive%20Component%20Object%20Reference) (OtherBodyIndex :type Integer) (bFromSweep :type Boolean) (SweepResult :type Hit%20Result%20Structure%20%28by%20ref%29))
  (if (== (Utilities|GetClass OtherActor) "/Game/_Game/Player/BP_PlayerCharacter.BP_PlayerCharacter_C")
    (if (Variables|Default|GetbIsClickable)
      (Development|PrintString "Hello")
      (CallFunction|Transfer))))

(event Custom|Transfer
  (bind _redcube (Variables|Default|GetredCube))
  (bind _returnvalue (Transformation|GetWorldLocation _redcube))
  (Transformation|Teleport (Math|Vector|MakeVector (.x _returnvalue) (.y _returnvalue) (+ (.z _returnvalue) 1e+01)) "0, 0, 0"))

(event EventBeginPlay)

(fn ConstructionScript)