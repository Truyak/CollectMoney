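; BP_SemiAutoTurret is an environment turret that fires BP_TurretBullet actors while a pawn is in its line of sight.
; A looping timer from BeginPlay drives a debug-drawn Pawn object trace forward from ShootPivot.
; A hit starts a second, slower looping timer to spawn bullets at the Nose location, and a miss clears it.
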(event Custom|CreateBullet
  (Game|SpawnActorfromClass "/Game/_Game/Blueprints/Environment/BP_TurretBullet.BP_TurretBullet_C" (Math|Transform|MakeTransform (Transformation|GetWorldLocation (Variables|Default|GetNose)) "0, 0, 0" "1.000000,1.000000,1.000000") "Undefined" "MultiplyWithRoot" 0 0))

(event Custom|Deneme
  (bind _shootpivot (Variables|Default|GetShootPivot))
  (bind _returnvalue (Transformation|GetWorldLocation _shootpivot))
  (bind _returnvalue_2 (Collision|LineTraceForObjects _returnvalue (+ _returnvalue (* (Math|Vector|GetForwardVector _shootpivot) (Variables|Default|GetTraceDistance))) (Utilities|Array|MakeArray "ObjectTypeQuery3") false 0 "ForDuration"))
  (if _returnvalue_2
    (if (not (Utilities|Time|IsValidTimerHandle (Variables|Default|GetTimerHandle)))
      (bind _returnvalue_3 (Utilities|Time|SetTimerbyEvent (EventDispatchers|CreateEvent :!event Custom|CreateBullet) 0.5 true true))
      (Variables|Default|SetTimerHandle _returnvalue_3))
    (elif (Utilities|Time|IsValidTimerHandle (Variables|Default|GetTimerHandle))
      (Utilities|Time|ClearandInvalidateTimerbyHandle (Variables|Default|GetTimerHandle)))))

(event EventBeginPlay
  (Utilities|Time|SetTimerbyEvent (EventDispatchers|CreateEvent :!event Custom|Deneme) 0.1 true true))

(fn ConstructionScript)