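; BP_InterpMovingColumns is an environmental hazard column that moves its Cube vertically and deals 100 damage to the player's health on box overlap.
; After a configurable start delay, downward and upward timelines are set up to hand off to each other in a loop, scaling their tracks by FloatingDistance.
; An InterpToMovement-style control-point setup remains disconnected in the construction script.
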(event OnComponentBeginOverlap(BoxCollision)
  (params (OverlappedComponent :type Primitive%20Component%20Object%20Reference) (OtherActor :type Actor%20Object%20Reference) (OtherComp :type Primitive%20Component%20Object%20Reference) (OtherBodyIndex :type Integer) (bFromSweep :type Boolean) (SweepResult :type Hit%20Result%20Structure%20%28by%20ref%29))
  (bind _asbp_player_character (Utilities|Casting|CastToBP_PlayerCharacter OtherActor))
  (Default|EventDecreaseHealth _asbp_player_character 100))

(event EventBeginPlay
  (Utilities|FlowControl|Delay (Variables|Default|GetDelayTime))
  (bind _downtrack (Timeline|DownsideMovementTimeline PlayFromStart)
    (:Update
      (Transformation|SetRelativeLocation (Variables|Default|GetCube) (Math|Vector|MakeVector 0.0 0.0 (* _downtrack (Variables|Default|GetFloatingDistance))) false false))
    (:Finished
      (Components|Timeline|PlayfromStart (Variables|Default|GetUpsideMovementTimeline)))))

(fn ConstructionScript)