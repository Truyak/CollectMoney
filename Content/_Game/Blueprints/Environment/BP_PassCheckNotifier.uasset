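; BP_PassCheckNotifier is an environment actor that detects a pawn passing in front of it and notifies the level's BP_ActivateLevel actor.
; BeginPlay starts a fast looping timer, apparently driving PassCheck, which sphere-traces for pawns a short distance along the Nose component's forward vector.
; Each hit looks up BP_ActivateLevel and calls Activation, with no guard against repeat calls in this graph.
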(event Custom|PassCheck
  (bind _nose (Variables|Default|GetNose))
  (bind _returnvalue (Transformation|GetWorldLocation _nose))
  (bind _returnvalue_2 (Collision|SphereTraceForObjects _returnvalue (+ _returnvalue (* (Math|Vector|GetForwardVector _nose) 5e+02)) 5e+01 (Utilities|Array|MakeArray "ObjectTypeQuery3") false 0 "None"))
  (if _returnvalue_2
    (bind _returnvalue_3 (Actor|GetActorOfClass "/Game/_Game/Blueprints/Environment/BP_ActivateLevel.BP_ActivateLevel_C"))
    (Default|Activation _returnvalue_3)))

(event EventBeginPlay
  (bind _returnvalue (Utilities|Time|SetTimerbyEvent (EventDispatchers|CreateEvent :!event Custom|PassCheck) 0.02 true true))
  (Variables|Default|SetTimerEvent _returnvalue))

(event Collision|EventActorBeginOverlap
  (params (OtherActor :type Actor%20Object%20Reference)))

(event EventTick
  (params (DeltaSeconds :type Float%20%28single-precision%29)))

(fn ConstructionScript)