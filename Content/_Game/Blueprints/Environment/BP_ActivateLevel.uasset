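; BP_ActivateLevel is an environment Blueprint that checks whether the player is allowed to pass when its Activation event is called.
; BeginPlay caches the BP_PlayerCharacter, and Activation reads that character's CanPass flag.
; On success, ReversePass clears the flag on the player, making the pass single-use.
; Both outcomes only print a message, with no level loading or other activation logic.
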(event Custom|Activation
  (Variables|Default|SetIs%20Passed (Variables|/Game/_Game/Player/BP_PlayerCharacter.BP_PlayerCharacter_C|GetbCanPass (Variables|Default|GetBP%20Player%20Character)))
  (if (Variables|Default|GetIs%20Passed)
    (Development|PrintString "Passed")
    (CallFunction|ReversePass)
    (else
      (Development|PrintString "Didnt Pass"))))

(event Custom|ReversePass
  (bind _output_get (Variables|Default|SetIs%20Passed false))
  (Variables|/Game/_Game/Player/BP_PlayerCharacter.BP_PlayerCharacter_C|SetbCanPass (Variables|Default|GetBP%20Player%20Character) _output_get))

(event EventBeginPlay
  (bind _asbp_player_character (Utilities|Casting|CastToBP_PlayerCharacter (Game|GetPlayerCharacter 0)))
  (Variables|Default|SetBP%20Player%20Character _asbp_player_character))

(fn ConstructionScript)