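; BP_LavaBlocksMovingVersion is an environment lava block meant to slide back and forth along its relative X axis.
; MoveTimeline scales its MoveTrack into the LavaBlock's relative location, and its Finished output flips between Play and Reverse for an endless ping-pong.
; Nothing starts the timeline: BeginPlay is a disabled stub and the construction script only calls its parent, so this graph never moves the block.
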(event EventBeginPlay
  (|CallParentFunction) ; This node is disabled and will not be called.\nDrag off pins to build functionality.
)

(fn ConstructionScript
  (|CallParentFunction))