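; BP_LaserBeam is a laser hazard that damages the player character on overlap with its box collision.
; A looping timer started on BeginPlay drives the beam update, which line-traces forward from an arrow component.
; The static mesh's Z scale follows the hit or trace-end distance, using only the world Y component, so sizing depends on orientation.
; Box overlap calls the player's decrease-health event independently of the trace.
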(event OnComponentBeginOverlap(BoxCollision)
  (params (OverlappedComponent :type Primitive%20Component%20Object%20Reference) (OtherActor :type Actor%20Object%20Reference) (OtherComp :type Primitive%20Component%20Object%20Reference) (OtherBodyIndex :type Integer) (bFromSweep :type Boolean) (SweepResult :type Hit%20Result%20Structure%20%28by%20ref%29))
  (bind _asbp_player_character (Utilities|Casting|CastToBP_PlayerCharacter OtherActor))
  (Default|EventDecreaseHealth _asbp_player_character (Variables|Default|GetDamageAmount)))

(event Custom|ShootLaserBeam
  (bind _arrow (Variables|Default|GetArrow))
  (bind _returnvalue (Transformation|GetWorldLocation _arrow))
  (bind (_outhit _returnvalue_2) (Class|KismetSystemLibrary|LineTraceSinglebyProfile _returnvalue (+ _returnvalue (* (Math|Vector|GetForwardVector _arrow) 2e+03)) "BlockAll" false 0 "None" true))
  (Transformation|SetRelativeScale3D (Variables|Default|GetStaticMesh) (Math|Vector|MakeVector 0.05 0.05 (.Y (Math|Vector|BreakVector (* (/ (- (select _returnvalue_2 (.Location (Collision|BreakHitResult _outhit)) (.TraceEnd (Collision|BreakHitResult _outhit))) (.TraceStart (Collision|BreakHitResult _outhit))) 495.441169) 0.991))))))

(event EventBeginPlay
  (Utilities|Time|SetTimerbyEvent (EventDispatchers|CreateEvent :!event Custom|ShootLaserBeam) 0.1 true true))

(event Collision|EventActorBeginOverlap
  (params (OtherActor :type Actor%20Object%20Reference)))

(event EventTick
  (params (DeltaSeconds :type Float%20%28single-precision%29)))

(fn ConstructionScript)